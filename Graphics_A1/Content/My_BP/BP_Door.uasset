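; BP_Door is a door that slides along its local Z axis when enough linked buttons are active.
; ButtonActivated and ButtonDeactivated events raise or lower an active count and compare it to ButtonNeeded.
; The DoorActivation timeline plays when the threshold is met and reverses otherwise, driving the Door component's relative Z position.
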(event `Button Activated`
  (`/Engine/EditorBlueprintResources/StandardMacros.IncrementInt` (`self.ButtonActive`)
    (:`  `
      (if (>= (`self.ButtonActive`) (`self.ButtonNeeded`))
        (bind (_direction _door_position) (`Timeline|Door Activation` :!label _label)
          (:`Update`
            (`SceneComponent.K2_SetRelativeLocation` (`self.Door`) (`KismetMathLibrary.MakeVector` 0.0 0.0 _door_position) false false)))
        (else
          (goto _label :!via `Reverse`))))))

(event `Button Deactivated`
  (`/Engine/EditorBlueprintResources/StandardMacros.DecrementInt` (`self.ButtonActive`)
    (:`  `
      (if (>= (`self.ButtonActive`) (`self.ButtonNeeded`))
        (goto _label)
        (else
          (goto _label :!via `Reverse`))))))

(fn `UserConstructionScript`)