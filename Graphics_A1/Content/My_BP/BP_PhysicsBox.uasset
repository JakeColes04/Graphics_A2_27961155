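; BP_PhysicsBox is a physics-simulated box that returns to its starting point when it hits an actor tagged Hazard.
; On BeginPlay it stores the actor location as the respawn point.
; On a Hazard hit it turns off physics on PhysBox, moves it to that point, then re-enables physics after a short delay.
; The reset sets location only, leaving rotation as it was.
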(event `self.ReceiveBeginPlay`
  (set `self.RespawnLocation` (`self.K2_GetActorLocation`)))

(event `self.PhysBox.OnComponentHit`
  (params (HitComponent :type "PrimitiveComponent Object Reference") (OtherActor :type "Actor Object Reference") (OtherComp :type "PrimitiveComponent Object Reference") (NormalImpulse :type "Vector Structure") (Hit :type "HitResult Structure (by ref)"))
  (bind _physbox (`self.PhysBox`))
  (if (`self.ActorHasTag` OtherActor "Hazard")
    (`PrimitiveComponent.SetSimulatePhysics` _physbox false)
    (`SceneComponent.K2_SetWorldLocation` _physbox (`self.RespawnLocation`) false false)
    (`KismetSystemLibrary.Delay` 0.1)
    (`PrimitiveComponent.SetSimulatePhysics` _physbox true)))

(fn `UserConstructionScript`)